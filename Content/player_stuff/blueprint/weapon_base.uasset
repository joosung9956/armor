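; Base weapon Blueprint whose fire event shoots a Bullet from the skeletal mesh's Muzzle socket.
; The Bullet spawns at the socket's world transform and always spawns regardless of collision.
; A muzzle flash emitter plays at the same socket with its yaw turned a quarter turn, followed by a debug "Hello" print.
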(event `fire`
  (bind _skeletalmesh (`self.SkeletalMesh`))
  (`|SpawnActorFromClass` "/Game/player_stuff/blueprint/Bullet.Bullet_C" (`SceneComponent.GetSocketTransform` (`self.SkeletalMesh`) "Muzzle" "RTS_World") "AlwaysSpawn" "OverrideRootScale")
  (`GameplayStatics.SpawnEmitterAtLocation` "/Game/InfinityBladeEffects/Effects/FX_Monsters/FX_Monster_Gruntling/Master/P_BackPack_MuzzleFlash2.P_BackPack_MuzzleFlash2" (`SceneComponent.GetSocketLocation` _skeletalmesh "Muzzle") (`KismetMathLibrary.MakeRotator` (.roll (`SceneComponent.GetSocketRotation` _skeletalmesh "Muzzle")) (.pitch (`SceneComponent.GetSocketRotation` _skeletalmesh "Muzzle")) (+ (.yaw (`SceneComponent.GetSocketRotation` _skeletalmesh "Muzzle")) -90.0)))
  (`KismetSystemLibrary.PrintString` "Hello"))

(fn `UserConstructionScript`)