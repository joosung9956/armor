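; Destructible monkey actor that breaks apart after taking repeated hits from bulletforDM projectiles.
; The Destructible component's hit event ignores other actors and increments a stack counter for each bullet hit.
; Once the counter has reached five, further bullet hits turn off physics simulation and apply radius damage with an impulse at the impact point to fracture the mesh.
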(event `self.Destructible.OnComponentHit`
  (params (HitComponent :type "PrimitiveComponent Object Reference") (OtherActor :type "Actor Object Reference") (OtherComp :type "PrimitiveComponent Object Reference") (NormalImpulse :type "Vector Structure") (Hit :type "HitResult Structure (by ref)"))
  (cast `/Game/player_stuff/blueprint/bulletforDM` OtherActor)
  (if (>= (`self.5번스택이쌓였으면`) 5.0)
    (`PrimitiveComponent.SetSimulatePhysics` (`self.Destructible`) false)
    (`DestructibleComponent.ApplyRadiusDamage` (`self.Destructible`) 10.0 (`.ImpactPoint` (`GameplayStatics.BreakHitResult` Hit)) 60.0 300.0 false)
    (else
      (set `self.5번스택이쌓였으면` (+ (`self.5번스택이쌓였으면`) 1.0)))))

(fn `UserConstructionScript`)